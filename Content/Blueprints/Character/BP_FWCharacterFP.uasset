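; First-person player character Blueprint that restores a stable position on spawn and spends stamina on movement.
; On possession it switches the first player controller to game-only input, and on BeginPlay it teleports to the StablePositionUpdater's StablePosition and prints it.
; The Enhanced Input Move action subtracts its TriggeredSeconds from PlayerStats.Stamina on each event, with no clamp in this graph.
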(event Input|EnhancedActionEvents|EnhancedInputActionMove
  (params (ActionValue :type Vector%202D%20Structure) (ElapsedSeconds :type Float%20%28double-precision%29) (TriggeredSeconds :type Float%20%28double-precision%29) (InputAction :type Input%20Action%20Object%20Reference :default "/Game/Blueprints/Inputs/Move.Move"))
  (bind _playerstats (Variables|Default|GetPlayerStats))
  (Variables|/Script/FireWorld.PlayerStatsComponent|SetStamina _playerstats (- (Variables|/Script/FireWorld.PlayerStatsComponent|GetStamina _playerstats) TriggeredSeconds)))

(event EventPossessed
  (params (NewController :type Controller%20Object%20Reference))
  (Input|SetInputModeGameOnly (Game|GetPlayerController 0) false))

(event EventBeginPlay
  (bind _stablepositionupdater (Variables|Default|GetStablePositionUpdater))
  (bind _stableposition (Variables|/Script/FireWorld.StablePositionUpdater|GetStablePosition _stablepositionupdater))
  (Transformation|SetActorTransform _stableposition false true)
  (Development|PrintString (Utilities|String|ToString(Transform) _stableposition)))

(fn ConstructionScript
  (|CallParentFunction))