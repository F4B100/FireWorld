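; Rocket projectile actor that explodes on hit, damaging nearby first-person characters and then destroying itself.
; The Hit event scans every BP_FWCharacterFP and compares its distance from the impact point to the explosion size.
; Those in range take explosion strength scaled by linear falloff, a hand-built radial damage with no line-of-sight check.
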(event Collision|EventHit
  (params (MyComp :type Primitive%20Component%20Object%20Reference) (Other :type Actor%20Object%20Reference) (OtherComp :type Primitive%20Component%20Object%20Reference) (bSelfMoved :type Boolean) (HitLocation :type Vector :default "0, 0, 0") (HitNormal :type Vector :default "0, 0, 0") (NormalImpulse :type Vector :default "0, 0, 0") (Hit :type Hit%20Result%20Structure%20%28by%20ref%29))
  (bind _rocket_explosion_size (Variables|Default|GetRocket%20Explosion%20Size))
  (bind _outactors (Actor|GetAllActorsOfClass "/Game/Blueprints/Character/BP_FWCharacterFP.BP_FWCharacterFP_C"))
  (for _array_element _outactors
    (if (<= (Math|Vector|VectorLength (- (.Location (Math|Transform|BreakTransform (Transformation|GetActorTransform _array_element))) (.Location (Collision|BreakHitResult Hit)))) _rocket_explosion_size)
      (Game|Damage|ApplyDamage _array_element (* (Variables|Default|GetRocket%20Explosion%20Strength) (/ (- _rocket_explosion_size (Math|Vector|VectorLength (- (.Location (Math|Transform|BreakTransform (Transformation|GetActorTransform _array_element))) (.Location (Collision|BreakHitResult Hit))))) _rocket_explosion_size)) (Variables|Default|GetController) self "/Script/Engine.DamageType")))
  (Actor|DestroyActor))

(fn ConstructionScript)