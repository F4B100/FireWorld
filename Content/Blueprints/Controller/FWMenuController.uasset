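; FWMenuController is a player controller that sets up mouse-driven menu input.
; On BeginPlay, when not running as the server, it casts its HUD to FWMenuHUD and gives UI-only input focus to that HUD's current menu, then shows the mouse cursor.
; A failed HUD cast only prints a debug message.
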(event EventBeginPlay
  (if (not (Networking|IsServer))
    (|Torunifnotserver)))

(fn ConstructionScript)