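; FWFPHUD is a HUD Blueprint that manages the on-screen menu widget for the first-person controller and character.
; On BeginPlay, only when IsServer is true, it caches BP_FWControllerFP and BP_FWCharacterFP, logging failed casts, then displays the ToDisplay widget and stores it as MainMenu.
; ChangeDisplayedMenu swaps menus by removing any current widget, creating the given class, adding it to the viewport and returning it.
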(event EventBeginPlay
  (bind _returnvalue (Game|Player|GetOwningPlayerController))
  (if (Networking|IsServer)
    (bind _asbp_fwcontroller_fp (Utilities|Casting|CastToBP_FWControllerFP _returnvalue)
      (:then
        (Variables|Default|SetController _asbp_fwcontroller_fp)
        (bind _asbp_fwcharacter_fp (Utilities|Casting|CastToBP_FWCharacterFP (Pawn|GetControlledPawn _returnvalue))
          (:then
            (Variables|Default|SetCharacter _asbp_fwcharacter_fp)
            (bind _created_widget (CallFunction|ChangeDisplayedMenu (Variables|Menu|GetToDisplay)))
            (bind _asbase_player_widget (Utilities|Casting|CastToBasePlayerWidget _created_widget))
            (Variables|Default|SetMainMenu _asbase_player_widget))
          (:CastFailed
            (Utilities|String|LogString "Could not cast Pawn to BP_FWCharacterFP in FWFPHUD"))))
      (:CastFailed
        (Utilities|String|LogString "Could not cast Controller to BP_FWControllerFP in FWFPHUD")))))

(fn ConstructionScript)

(fn ChangeDisplayedMenu
  (params (New%20Menu :type User%20Widget%20Class%20Reference))
  (if (Utilities|IsValid (Variables|Default|GetCurrent%20Menu))
    (Widget|RemovefromParent (Variables|Default|GetCurrent%20Menu)))
  (bind _returnvalue (UserInterface|CreateWidget New%20Menu))
  (bind _output_get (Variables|Default|SetCurrent%20Menu _returnvalue))
  (UserInterface|Viewport|AddtoViewport _output_get 0)
  (return _output_get))