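; Menu HUD that creates and shows a configurable menu widget on BeginPlay, skipped when running as server.
; ChangeDisplayedMenu removes any valid current menu, creates a widget of the given class, adds it to the viewport and returns it.
; BeginPlay passes the ToDisplay class to that function and stores the result as MainMenu, while CurrentMenu tracks whichever menu was last displayed.
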(event EventBeginPlay
  (if (not (Networking|IsServer))
    (bind _created_widget (CallFunction|ChangeDisplayedMenu (Variables|Menu|GetToDisplay)))
    (Variables|Default|SetMainMenu _created_widget)))

(fn ConstructionScript)

(fn ChangeDisplayedMenu
  (params (New%20Menu :type User%20Widget%20Class%20Reference))
  (if (Utilities|IsValid (Variables|Default|GetCurrent%20Menu))
    (Widget|RemovefromParent (Variables|Default|GetCurrent%20Menu)))
  (bind _returnvalue (UserInterface|CreateWidget New%20Menu))
  (bind _output_get (Variables|Default|SetCurrent%20Menu _returnvalue))
  (UserInterface|Viewport|AddtoViewport _output_get 0)
  (return _output_get))